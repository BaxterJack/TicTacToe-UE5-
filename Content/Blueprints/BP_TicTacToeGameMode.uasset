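; Tic-Tac-Toe game mode Blueprint that drives the on-screen display for turns, scores, game over and series over.
; BeginPlay creates the WBP_GameUI widget, adds it to the viewport and shows the current player's turn.
; Update events forward state to that widget, with no game rules in these graphs.
; Wins show a gold line between supplied positions through the nested WBPWinLine widget, which restart hides.
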(event `self.ReceiveBeginPlay`
  (`self.SetGameUI`)
  (`/Game/UI/WBP_GameUI.SetTurnTextCurrentPlayer` (`self.GameUI`) (`self.CurrentPlayer`)))

(event `self.UpdateTurnDisplay`
  (params (Player :type Integer))
  (`/Game/UI/WBP_GameUI.SetTurnTextCurrentPlayer` (`self.GameUI`) Player))

(event `self.UpdateRestartDisplay`
  (`/Game/UI/WBP_GameUI.ResetDisplay` (`self.GameUI`))
  (`Widget.SetVisibility` (`/Game/UI/WBP_GameUI.WBP_WinLine` (`self.GameUI`)) "Hidden"))

(event `self.UpdateGameOverDisplay`
  (params (WinningPlayer :type Integer) (InStartPos :type "Vector Structure") (InEndPos :type "Vector Structure"))
  (bind _gameui (`self.GameUI`))
  (bind _wbp_winline (`/Game/UI/WBP_GameUI.WBP_WinLine` (`self.GameUI`)))
  (`/Game/UI/WBP_GameUI.ShowGameOver` _gameui WinningPlayer)
  (`/Game/UI/WBP_GameUI.SetTurnTextRestart Game` _gameui)
  (`Widget.SetVisibility` _wbp_winline "Visible")
  (`/Game/UI/WBP_WinLine.ShowLine` _wbp_winline InStartPos InEndPos (struct :`R` 1.0 :`G` 0.8 :`A` 1.0)))

(event `self.UpdateScoreDisplay`
  (params (P1Score :type Integer) (P2Score :type Integer))
  (`/Game/UI/WBP_GameUI.UpdateScores` (`self.GameUI`) P1Score P2Score))

(event `self.UpdateSeriesOverDisplay`
  (params (WinningPlayer :type Integer) (InStartPos :type "Vector Structure") (InEndPos :type "Vector Structure"))
  (bind _wbp_winline (`/Game/UI/WBP_GameUI.WBP_WinLine` (`self.GameUI`)))
  (`/Game/UI/WBP_GameUI.ShowSeriesOver` (`self.GameUI`) WinningPlayer)
  (`Widget.SetVisibility` _wbp_winline "Visible")
  (`/Game/UI/WBP_WinLine.ShowLine` _wbp_winline InStartPos InEndPos (struct :`R` 1.0 :`G` 0.8 :`A` 1.0)))

(fn `SetGameUI`
  (bind _returnvalue (`|CreateWidget` "/Game/UI/WBP_GameUI.WBP_GameUI_C" (`GameplayStatics.GetPlayerController` 0)))
  (`UserWidget.AddToViewport` _returnvalue 0)
  (set `self.GameUI` _returnvalue))

(fn `UserConstructionScript`)